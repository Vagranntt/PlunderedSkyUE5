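; BP_ActortoSpawn is a collectible orb that is picked up when a Character overlaps its Box.
; Overlap enables input and immediately calls CollectOrb, and end overlap disables input, though the graph contains no input events.
; CollectOrb decrements CollectiblesLeft on BP_ThirdPersonGameMode, adds a newly created BP_WidgetCollection to the viewport, then destroys the actor.
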(event OnComponentBeginOverlap(Box)
  (params (OverlappedComponent :type Primitive%20Component%20Object%20Reference) (OtherActor :type Actor%20Object%20Reference) (OtherComp :type Primitive%20Component%20Object%20Reference) (OtherBodyIndex :type Integer) (bFromSweep :type Boolean) (SweepResult :type Hit%20Result%20Structure%20%28by%20ref%29))
  (Utilities|Casting|CastToCharacter OtherActor)
  (Input|EnableInput (Game|GetPlayerController 0))
  (CallFunction|CollectOrb))

(event OnComponentEndOverlap(Box)
  (params (OverlappedComponent :type Primitive%20Component%20Object%20Reference) (OtherActor :type Actor%20Object%20Reference) (OtherComp :type Primitive%20Component%20Object%20Reference) (OtherBodyIndex :type Integer))
  (Utilities|Casting|CastToCharacter OtherActor)
  (Input|DisableInput (Game|GetPlayerController 0)))

(event Custom|CollectOrb
  (bind _asbp_third_person_game_mode (Utilities|Casting|CastToBP_ThirdPersonGameMode (Game|GetGameMode)))
  (bind _result (Math|Integer|DecrementInt (Variables|/Game/ThirdPerson/Blueprints/BP_ThirdPersonGameMode.BP_ThirdPersonGameMode_C|GetCollectiblesLeft _asbp_third_person_game_mode))
    (:%20%20
      (Variables|/Game/ThirdPerson/Blueprints/BP_ThirdPersonGameMode.BP_ThirdPersonGameMode_C|SetCollectiblesLeft _asbp_third_person_game_mode _result)
      (bind _returnvalue (UserInterface|CreateWidget "/Game/UI/Widgets/BP_WidgetCollection.BP_WidgetCollection_C"))
      (UserInterface|Viewport|AddtoViewport _returnvalue 0)
      (Actor|DestroyActor))))

(fn ConstructionScript)